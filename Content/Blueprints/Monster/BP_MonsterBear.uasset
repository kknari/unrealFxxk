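; Bear monster character driven by a state machine (Locomotion, Chase, Attack, Dead) that sets walk speed and broadcasts each state change.
; While attacks are allowed, PawnSensing starts a chase; losing the target beyond sight radius or player death returns it to Locomotion.
; A toggleable attack collision deals damage on overlap.
; Taking damage plays a timeline-driven material effect, or at zero health disables capsule collision and schedules removal.
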(event OnSeePawn(PawnSensing)
  (params (Pawn :type Pawn%20Object%20Reference))
  (if (Variables|Default|GetCanAttack)
    (switch Utilities|FlowControl|Switch|SwitchonEBearState "NewEnumerator0"
      (:NewEnumerator0
        (Variables|Actor|SetInstigator Pawn)
        (CallFunction|SetState "NewEnumerator1")))))

(event OnComponentBeginOverlap(AttackCollision)
  (params (OverlappedComponent :type Primitive%20Component%20Object%20Reference) (OtherActor :type Actor%20Object%20Reference) (OtherComp :type Primitive%20Component%20Object%20Reference) (OtherBodyIndex :type Integer) (bFromSweep :type Boolean) (SweepResult :type Hit%20Result%20Structure%20%28by%20ref%29))
  (Game|Damage|ApplyDamage OtherActor 2e+01 (Pawn|GetController) self))

(event Custom|SetState
  (params (NewState :type EBearState%20Enum :default "NewEnumerator0"))
  (bind _charactermovement (Variables|Character|GetCharacterMovement))
  ;[1 1 1] 상태 변경 이벤트
  (if (not (Utilities|Enum|Equal(Enum) (Variables|Default|GetState) "NewEnumerator3"))
    (bind _output_get (Variables|Default|SetState NewState))
    (Default|CallStateChangedEvent _output_get)
    (switch Utilities|FlowControl|Switch|SwitchonEBearState _output_get
      (:NewEnumerator0
        (Variables|/Script/Engine.CharacterMovementComponent|SetMaxWalkSpeed _charactermovement 2e+02))
      (:NewEnumerator1
        (Variables|/Script/Engine.CharacterMovementComponent|SetMaxWalkSpeed _charactermovement 5e+02))
      (:NewEnumerator2
        (Variables|/Script/Engine.CharacterMovementComponent|SetMaxWalkSpeed _charactermovement 0.0 :!label _label))
      (:NewEnumerator3
        (goto _label)))))

(event Custom|Play%20Damage%20Effect
  ;[1 1 1] 데미지 머터리얼 이펙트 재생
  (bind _alpha (Timeline|Damage%20Effect PlayFromStart)
    (:Update
      (Rendering|Material|SetScalarParameterValueonMaterials (Variables|Character|GetMesh) "DamageFactor" _alpha))))

(event Custom|Collision%20On
  (Collision|SetCollisionEnabled (Variables|Default|GetAttack%20Collision) "QueryOnly"))

(event Custom|Collision%20Off
  (Collision|SetCollisionEnabled (Variables|Default|GetAttack%20Collision) "NoCollision"))

(event Custom|Check%20Distance%20to%20Player
  ;[1 1 1] 플레이어가 시야에서 벗어났는지 확인하고, 벗어났으면 다시 정찰 모드로 변경
  (Utilities|IsValid (Variables|Actor|GetInstigator)
    (:Is%20Valid
      (if (> (Math|Vector|Distance(Vector) (Transformation|GetActorLocation (Variables|Actor|GetInstigator)) (Transformation|GetActorLocation)) (Variables|/Script/AIModule.PawnSensingComponent|GetSightRadius (Variables|Default|GetPawnSensing)))
        (Variables|Actor|SetInstigator 0)
        (CallFunction|SetState "NewEnumerator0")))))

(event Custom|OnplayerDead
  (Variables|Default|SetCanAttack false)
  (Variables|Actor|SetInstigator 0)
  (CallFunction|SetState "NewEnumerator0"))

(event EventBeginPlay
  (CallFunction|SetState "NewEnumerator0")
  (Collision|SetCollisionEnabled (Variables|Default|GetAttack%20Collision) "NoCollision")
  (bind _asbp_player_state (Utilities|Casting|CastToBP_PlayerState (Game|GetPlayerState 0)))
  (EventDispatchers|BindEventtoOnPlayerDead _asbp_player_state (delegate Custom|OnplayerDead)))

(event Collision|EventActorBeginOverlap
  (params (OtherActor :type Actor%20Object%20Reference)))

(event Game|Damage|EventAnyDamage
  (params (Damage :type Float%20%28single-precision%29) (DamageType :type Damage%20Type%20Object%20Reference) (InstigatedBy :type Controller%20Object%20Reference) (DamageCauser :type Actor%20Object%20Reference))
  ;[1 1 1] 데미지 처리 이벤트
  ;;[1 1 1] 죽었는지 확인 - 죽었을 땐 처리 무시
  (if (not (Utilities|Enum|Equal(Enum) (Variables|Default|GetState) "NewEnumerator3"))
    ;;[1 1 1] 데미지 처리
    (Variables|Default|SetHealth%20Power (- (Variables|Default|GetHealth%20Power) Damage))
    ;;[1 1 1] 생사 여부 판단
    (if (> (Variables|Default|GetHealth%20Power) 0.0)
      ;;[1 1 1] 살았을 때는 데미지 효과 재생
      (CallFunction|PlayDamageEffect)
      (else
        ;;[1 1 1] 죽었을 때 처리 - 상태변경/콜리전 끄기/액터 삭제 예약
        (CallFunction|SetState "NewEnumerator3")
        (Collision|SetCollisionEnabled (Variables|Collision|GetCapsuleComponent) "NoCollision")
        (Actor|SetLifeSpan 5.0)))))

(event EventTick
  (params (DeltaSeconds :type Float%20%28single-precision%29))
  (switch Utilities|FlowControl|Switch|SwitchonEBearState (Variables|Default|GetState)
    (:NewEnumerator1
      _)
    (:NewEnumerator2
      _))
  (CallFunction|CheckDistancetoPlayer))

(fn ConstructionScript)