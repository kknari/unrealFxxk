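; AI controller that drives the bear monster through the monster Behavior Tree and Blackboard.
; On possess it sets up the Blackboard with a patrol time and the pawn's start location, runs the tree, then binds to the bear's state-changed event.
; Each state change is mirrored into the Blackboard, and entering Chase also stores the pawn's Instigator as the target player.
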(event Custom|Bear%20State%20Changed
  (params (NewState :type EBearState%20Enum :default "NewEnumerator0"))
  (AI|Components|Blackboard|SetValueasEnum (Variables|Default|GetBlackboard) (Variables|Default|GetState%20Key%20Name) NewState)
  (switch Utilities|FlowControl|Switch|SwitchonEBearState NewState
    (:NewEnumerator1
      (AI|Components|Blackboard|SetValueasObject (Variables|Default|GetBlackboard) (Variables|Default|GetTargetPlayer%20KeyName) (Variables|/Script/Engine.Actor|GetInstigator (Pawn|GetControlledPawn))))))

(event EventBeginPlay)

(event EventTick
  (params (DeltaSeconds :type Float%20%28single-precision%29)))

(event EventPossess
  (params (PossessedPawn :type Pawn%20Object%20Reference))
  (Utilities|FlowControl|Sequence
    (:then_0
      (Class|AIController|UseBlackboard "/Game/Blueprints/Monster/AI/BP_MonsterBB.BP_MonsterBB")
      (AI|Components|Blackboard|SetValueasFloat (Variables|Default|GetBlackboard) (Variables|Default|GetPatrol%20Time%20Name) 3.0)
      (AI|Components|Blackboard|SetValueasVector (Variables|Default|GetBlackboard) (Variables|Default|GetStart%20Location%20Name) (Transformation|GetActorLocation (Pawn|GetControlledPawn))))
    (:then_1
      (AI|RunBehaviorTree "/Game/Blueprints/Monster/AI/BP_MonsterBT.BP_MonsterBT"))
    (:then_2
      (bind _asbp_monster_bear (Utilities|Casting|CastToBP_MonsterBear PossessedPawn))
      (EventDispatchers|BindEventtoStateChangedEvent _asbp_monster_bear (delegate Custom|Bear%20State%20Changed)))))

(fn ConstructionScript)