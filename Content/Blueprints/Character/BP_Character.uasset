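; BP_Character is a player character Blueprint that handles movement, camera look and jumping through Enhanced Input.
; BeginPlay adds the IMC_CharacterMove mapping context to player controller 0's input subsystem.
; Move input strafes along the control rotation's right vector and moves forward along a yaw-only forward vector, so camera pitch does not affect it.
; Look input drives controller yaw and pitch, while jump press and release start and stop jumping.
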(event Input|EnhancedActionEvents|EnhancedInputActionIA_CharacterJump
  (params (ActionValue :type Boolean) (ElapsedSeconds :type Float%20%28double-precision%29) (TriggeredSeconds :type Float%20%28double-precision%29) (InputAction :type Input%20Action%20Object%20Reference :default "/Game/Blueprints/Character/IA_CharacterJump.IA_CharacterJump"))
  ;[1 1 1] 캐릭터 점프
  (:Started
    (Character|Jump))
  (:Completed
    (Character|StopJumping)))

(event Input|EnhancedActionEvents|EnhancedInputActionIA_CharacterMove
  (params (ActionValue :type Vector%202D%20Structure) (ElapsedSeconds :type Float%20%28double-precision%29) (TriggeredSeconds :type Float%20%28double-precision%29) (InputAction :type Input%20Action%20Object%20Reference :default "/Game/Blueprints/Input/IA_CharacterMove.IA_CharacterMove"))
  ;[1 1 1] 캐릭터 이동
  (:Triggered
    (Pawn|Input|AddMovementInput (Math|Vector|GetRightVector (Pawn|GetControlRotation :!class /Script/Engine.Pawn)) (.x ActionValue) false)
    (Pawn|Input|AddMovementInput (Math|Vector|GetForwardVector (Math|Rotator|MakeRotator 0.0 0.0 (.yaw (Pawn|GetControlRotation :!class /Script/Engine.Pawn)))) (.y ActionValue) false)))

(event Input|EnhancedActionEvents|EnhancedInputActionIA_CameraRotate
  (params (ActionValue :type Vector%202D%20Structure) (ElapsedSeconds :type Float%20%28double-precision%29) (TriggeredSeconds :type Float%20%28double-precision%29) (InputAction :type Input%20Action%20Object%20Reference :default "/Game/Blueprints/Character/IA_CameraRotate.IA_CameraRotate"))
  (:Triggered
    (Pawn|Input|AddControllerYawInput (.x ActionValue))
    (Pawn|Input|AddControllerPitchInput (.y ActionValue))))

(event EventBeginPlay
  ;[1 1 1] 입력을 사용한다고 설정하는 부분(꼭 필요)
  (Input|AddMappingContext (PlayerController|LocalPlayerSubsystems|GetEnhancedInputLocalPlayerSubsystem (Game|GetPlayerController 0)) "/Game/Blueprints/Input/IMC_CharacterMove.IMC_CharacterMove" 0 "(bIgnoreAllPressedKeysUntilRelease=True,bForceImmediately=False)"))

(fn ConstructionScript)