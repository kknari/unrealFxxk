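; BP_Warior is the player warrior character, with movement, camera look and a montage-based melee combo.
; The jump input triggers Attack, which plays the montage or, if already playing, sets ComboSection from the current section.
; CollisionOn/Off toggle the weapon hitbox, whose overlaps apply fixed damage.
; Damage taken is forwarded to BP_PlayerState, whose death event sets state, disables collision, zeroes walk speed and switches to UI-only input.
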(event OnComponentBeginOverlap(WeaponCollision)
  (params (OverlappedComponent :type Primitive%20Component%20Object%20Reference) (OtherActor :type Actor%20Object%20Reference) (OtherComp :type Primitive%20Component%20Object%20Reference) (OtherBodyIndex :type Integer) (bFromSweep :type Boolean) (SweepResult :type Hit%20Result%20Structure%20%28by%20ref%29))
  (Game|Damage|ApplyDamage OtherActor 3e+01 (Pawn|GetController) self))

(event Custom|Attack
  ;[1 1 1] 공격 시작&종료
  (CallFunction|SetState "NewEnumerator1")
  ;[1 1 1] 몽타주 재생 중인지 확인
  (if (Animation|Montage|MontageIsPlaying (Components|SkeletalMesh|GetAnimInstance (Variables|Character|GetMesh)) "/Game/Blueprints/Character/Warrior_AnimMontage.Warrior_AnimMontage")
    ;[1 1 1] 콤보 공격 처리
    (switch name (Animation|Montage|MontageGetCurrentSection (Components|SkeletalMesh|GetAnimInstance (Variables|Character|GetMesh)) "/Game/Blueprints/Character/Warrior_AnimMontage.Warrior_AnimMontage")
      (:Attack1
        (Variables|Default|SetComboSection "Attack2"))
      (:Attack2
        (Variables|Default|SetComboSection "Attack3"))
      (:Attack3
        (Variables|Default|SetComboSection "Attack4")))
    (else
      ;[1 1 1] 몽타주 재생 - 공격 애니메이션 재생
      (Animation|Montage|MontagePlay (Components|SkeletalMesh|GetAnimInstance (Variables|Character|GetMesh)) "/Game/Blueprints/Character/Warrior_AnimMontage.Warrior_AnimMontage" 1.0 "MontageLength" 0.0 true))))

(event Custom|AttackEnd
  ;[1 1 1] 공격 시작&종료
  (CallFunction|SetState "NewEnumerator0")
  (Variables|Default|SetComboSection "None"))

(event Custom|SetState
  (params (NewState :type EWarriorState%20Enum :default "NewEnumerator0"))
  ;[1 1 1] 캐릭터 상태 변경 이벤트
  (Variables|Default|SetState NewState))

(event Custom|CollisionOn
  ;[1 1 1] 공격 판정 시작&종료
  (Collision|SetCollisionEnabled (Variables|Default|GetWeaponCollision) "QueryOnly")
  (Development|PrintString "On"))

(event Custom|CollisionOff
  ;[1 1 1] 공격 판정 시작&종료
  (Collision|SetCollisionEnabled (Variables|Default|GetWeaponCollision) "NoCollision")
  (Development|PrintString "Off"))

(event Custom|OnPlayerDead
  ;[1 1 1] 플레이어 사망처리
  (CallFunction|SetState "NewEnumerator2")
  (Collision|SetCollisionEnabled (Variables|Collision|GetCapsuleComponent) "NoCollision")
  (Collision|SetCollisionEnabled (Variables|Default|GetWeaponCollision) "NoCollision")
  (Variables|/Script/Engine.CharacterMovementComponent|SetMaxWalkSpeed (Variables|Character|GetCharacterMovement) 0.0)
  (Input|SetInputModeUIOnly (Game|GetPlayerController 0) 0 "DoNotLock" false))

(event Input|EnhancedActionEvents|EnhancedInputActionIA_CameraRotate
  (params (ActionValue :type Vector%202D%20Structure) (ElapsedSeconds :type Float%20%28double-precision%29) (TriggeredSeconds :type Float%20%28double-precision%29) (InputAction :type Input%20Action%20Object%20Reference :default "/Game/Blueprints/Character/IA_CameraRotate.IA_CameraRotate"))
  ;[1 1 1] 카메라 회전
  (:Triggered
    (Pawn|Input|AddControllerYawInput (.x ActionValue))
    (Pawn|Input|AddControllerPitchInput (.y ActionValue))))

(event Input|EnhancedActionEvents|EnhancedInputActionIA_CharacterMove
  (params (ActionValue :type Vector%202D%20Structure) (ElapsedSeconds :type Float%20%28double-precision%29) (TriggeredSeconds :type Float%20%28double-precision%29) (InputAction :type Input%20Action%20Object%20Reference :default "/Game/Blueprints/Input/IA_CharacterMove.IA_CharacterMove"))
  ;[1 1 1] 캐릭터 이동
  (:Triggered
    (Pawn|Input|AddMovementInput (Math|Vector|GetRightVector (Pawn|GetControlRotation :!class /Script/Engine.Pawn)) (.x ActionValue) false)
    (Pawn|Input|AddMovementInput (Math|Vector|GetForwardVector (Math|Rotator|MakeRotator 0.0 0.0 (.yaw (Pawn|GetControlRotation :!class /Script/Engine.Pawn)))) (.y ActionValue) false)))

(event Input|EnhancedActionEvents|EnhancedInputActionIA_CharacterJump
  (params (ActionValue :type Boolean) (ElapsedSeconds :type Float%20%28double-precision%29) (TriggeredSeconds :type Float%20%28double-precision%29) (InputAction :type Input%20Action%20Object%20Reference :default "/Game/Blueprints/Character/IA_CharacterJump.IA_CharacterJump"))
  (:Started
    (CallFunction|Attack)))

(event EventBeginPlay
  ;[1 1 1] 입력 선언
  (Input|AddMappingContext (PlayerController|LocalPlayerSubsystems|GetEnhancedInputLocalPlayerSubsystem (Game|GetPlayerController 0)) "/Game/Blueprints/Input/IMC_CharacterMove.IMC_CharacterMove" 0 "(bIgnoreAllPressedKeysUntilRelease=True,bForceImmediately=False)")
  (CallFunction|CollisionOff)
  ;[1 1 1] 플레이어 사망처리
  (bind _asbp_player_state (Utilities|Casting|CastToBP_PlayerState (Game|GetPlayerState 0)))
  (EventDispatchers|BindEventtoOnPlayerDead _asbp_player_state (delegate Custom|OnPlayerDead)))

(event Collision|EventActorBeginOverlap
  (params (OtherActor :type Actor%20Object%20Reference)))

(event EventTick
  (params (DeltaSeconds :type Float%20%28single-precision%29)))

(event Game|Damage|EventAnyDamage
  (params (Damage :type Float%20%28single-precision%29) (DamageType :type Damage%20Type%20Object%20Reference) (InstigatedBy :type Controller%20Object%20Reference) (DamageCauser :type Actor%20Object%20Reference))
  (bind _asbp_player_state (Utilities|Casting|CastToBP_PlayerState (Game|GetPlayerState 0)))
  (Default|GetDamage _asbp_player_state Damage))

(fn ConstructionScript)